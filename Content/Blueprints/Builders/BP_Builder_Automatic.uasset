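; Builder actor that generates a vertical grid of instanced cubes in the construction script, with chosen blocks cut out by index.
; Row length, count, spacing and size shape the grid, and each cube gets an optional text label showing its instance index.
; DeleteBlocks is sorted ascending, then a running removal counter offsets each index as instances shift, and the matching labels are destroyed.
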(event EventBeginPlay)

(fn ConstructionScript
  (bind _cube (Variables|Default|GetCube))
  (CallFunction|SortDeleteBlocksArray)
  (for _index (range 0 (- (Math|Float|Ceil (/ (Math|Conversions|ToFloat(Integer) (Variables|Default|GetCount)) (Math|Conversions|ToFloat(Integer) (Variables|Default|GetRowLength)))) 1))
    (for _index_2 (range 0 (- (Variables|Default|GetRowLength) 1))
      (bind _returnvalue (Components|InstancedStaticMesh|AddInstance (Variables|Default|GetCube) (Math|Transform|MakeTransform (Math|Vector|MakeVector (* _index_2 (Variables|Default|GetBlockSpacing)) 0.0 (* _index (Variables|Default|GetBlockSpacing))) "0, 0, 0" (Math|Conversions|ToVector(Float) (/ (Variables|Default|GetBlockSize) 2e+02)))))
      (bind _returnvalue_2 (AddComponent|AddTextRenderComponent false (Math|Transform|MakeTransform (Math|Vector|MakeVector (* _index_2 (Variables|Default|GetBlockSpacing)) -1.1e+02 (* _index (Variables|Default|GetBlockSpacing))) "0,-90.000000, 0" "1,1,1")))
      (Utilities|Array|Add (Variables|Default|GetTextRenderArray) (Utilities|Struct|MakeFTextStruct _returnvalue_2 _returnvalue))
      (Rendering|Components|TextRender|SetText _returnvalue_2 (Utilities|Text|ToText(Integer) _returnvalue))
      (Rendering|Components|TextRender|SetTextRenderColor _returnvalue_2 (Variables|Default|GetText%20Color))
      (Rendering|SetVisibility _returnvalue_2 (Variables|Default|GetTextVisibility) false)))
  (for _array_element (Variables|Default|GetDeleteBlocks)
    (if (.ReturnValue (Components|InstancedStaticMesh|GetInstanceTransform _cube (- _array_element (Variables|Default|GetRemovalIndexCounter)) false))
      (Class|InstancedStaticMeshComponent|RemoveInstance _cube (- _array_element (Variables|Default|GetRemovalIndexCounter)))
      (for _array_element_2 (Variables|Default|GetTextRenderArray)
        (if (== (.instanceindex _array_element_2) _array_element)
          (Components|DestroyComponent (.textrendercomponent _array_element_2))))
      (Variables|Default|SetRemovalIndexCounter (+ (Variables|Default|GetRemovalIndexCounter) 1)))))

(fn SortDeleteBlocksArray
  (while (> (Utilities|Array|Length (Variables|Default|GetDeleteBlocks)) 0)
    (Utilities|Array|Insert (LocalVariables|GetDeleteBlocksSorted) (.MaxValue (Math|Integer|MaxOfIntArray (Variables|Default|GetDeleteBlocks))))
    (Utilities|Array|RemoveIndex (Variables|Default|GetDeleteBlocks) (.IndexOfMaxValue (Math|Integer|MaxOfIntArray (Variables|Default|GetDeleteBlocks)))))
  (Variables|Default|SetDeleteBlocks (LocalVariables|GetDeleteBlocksSorted)))