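; BP_Builder is a construction-script builder that lays out a grid of instanced copies of a chosen mesh.
; Nested row and column loops add instances along X and Z at a uniform Spacing, with no runtime logic.
; SortDeletedBlocks is called before the loops but does nothing: its DeleteBlocks sorting is disconnected, and no instances are removed.
; A per-cell text render component is also left unwired.
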(event EventBeginPlay)

(fn ConstructionScript
  (Components|StaticMesh|SetStaticMesh (Variables|Default|GetMesh) (Variables|Default|GetMeshes))
  (CallFunction|SortDeletedBlocks)
  (for _index (range 0 (- (Variables|Default|GetRows) 1))
    (for _index_2 (range 0 (- (Variables|Default|GetRowLength) 1))
      (Components|InstancedStaticMesh|AddInstance (Variables|Default|GetMesh) (Math|Transform|MakeTransform (Math|Vector|MakeVector (Math|Conversions|ToFloat(Integer) (* _index_2 (Variables|Default|GetSpacing))) 0.0 (Math|Conversions|ToFloat(Integer) (* _index (Variables|Default|GetSpacing)))) "0, 0, 0" "1,1,1")))))

(fn SortDeletedBlocks)